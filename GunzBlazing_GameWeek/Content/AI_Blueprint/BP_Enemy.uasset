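; BP_Enemy is a flipbook-sprite enemy that chases the first-person player once PawnSensing spots them.
; Projectile hits drain health; on death it swaps flipbook, stops, plays sound and particles, then destroys itself.
; It increments the game mode's living-enemy count on BeginPlay, then decrements it and triggers a remaining-enemy check on death.
; Attack is an empty stub with disconnected damage logic, and Tick pins rotation to zero.
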(event OnSeePawn(PawnSensing)
  (params (Pawn :type Pawn%20Object%20Reference))
  (bind _asbp_first_person_character (Utilities|Casting|CastToBP_FirstPersonCharacter Pawn))
  (Utilities|FlowControl|Sequence
    (:then_0
      (Variables|Default|SetCan%20See%20Enemy true)
      (AI|AIMoveTo self "0, 0, 0" _asbp_first_person_character 5.0 false))
    (:then_1
      (Utilities|FlowControl|RetriggerableDelay 0.6)
      (Variables|Default|SetCan%20See%20Enemy false))))

(event OnComponentHit(CapsuleComponent)
  (params (HitComponent :type Primitive%20Component%20Object%20Reference) (OtherActor :type Actor%20Object%20Reference) (OtherComp :type Primitive%20Component%20Object%20Reference) (NormalImpulse :type Vector :default "0, 0, 0") (Hit :type Hit%20Result%20Structure%20%28by%20ref%29))
  (Utilities|Casting|CastToBP_FirstPersonProjectile OtherActor)
  (CallFunction|TakeDamage 5.0 "None"))

(event Custom|Attack)

(event EventTakeDamage
  (params (Damage :type Float%20%28double-precision%29) (Bone :type Name :default "None"))
  ;[1 1 1] Take Damage
  (bind _output_get (Variables|Default|SetCurrent%20Health (- (Variables|Default|GetCurrent%20Health) Damage)))
  (if (<= _output_get 0.0)
    ;;[1 1 1] Animation Dead
    (Variables|Default|SetIs%20Dead true)
    (Sprite|SetFlipbook (Variables|Default|GetEnemy) (Variables|Default|GetFlipbook))
    (Variables|/Script/Engine.CharacterMovementComponent|SetMaxWalkSpeed (Variables|Character|GetCharacterMovement) 0.0)
    (Utilities|FlowControl|Delay 1.2)
    (Audio|PlaySound2D 0 1.0 1.0 0.0 0 0)
    (Effects|SpawnEmitteratLocation 0 "0, 0, 0")
    ;;[1 1 1] Conter
    (Utilities|FlowControl|DoOnce false
      (:Completed
        (bind _asbp_first_person_game_mode (Utilities|Casting|CastToBP_FirstPersonGameMode (Game|GetGameMode)))
        (Math|Integer|DecrementInt (Variables|/Game/FirstPerson/Blueprints/BP_FirstPersonGameMode.BP_FirstPersonGameMode_C|GetEnemyAlive _asbp_first_person_game_mode)
          (:%20%20
            (Default|CheckEnemyLeft _asbp_first_person_game_mode)
            (Actor|DestroyActor)))))))

(event EventBeginPlay
  (Variables|Default|SetCurrent%20Health (Variables|Default|GetMax%20Health))
  (bind _asbp_first_person_game_mode (Utilities|Casting|CastToBP_FirstPersonGameMode (Game|GetGameMode)))
  (Math|Integer|IncrementInt (Variables|/Game/FirstPerson/Blueprints/BP_FirstPersonGameMode.BP_FirstPersonGameMode_C|GetEnemyAlive _asbp_first_person_game_mode)))

(event Collision|EventActorBeginOverlap
  (params (OtherActor :type Actor%20Object%20Reference))
  (Utilities|Casting|CastToBP_FirstPersonCharacter OtherActor))

(event EventTick
  (params (DeltaSeconds :type Float%20%28single-precision%29))
  (Transformation|SetActorRotation "0, 0, 0"))

(event Collision|EventActorEndOverlap
  (params (OtherActor :type Actor%20Object%20Reference))
  (Utilities|Casting|CastToBP_FirstPersonCharacter OtherActor)
  (Variables|Default|SetIs%20Attacking false))

(fn ConstructionScript)